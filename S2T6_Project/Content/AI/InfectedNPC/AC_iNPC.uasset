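; AI controller for the infected NPC that starts its behavior tree and seeds it with patrol settings.
; On BeginPlay it runs BT_iNPC, casts the controlled pawn to iNPC and stores it.
; It then copies the pawn's patrol path looping flag and wait time into the blackboard, along with an initial forward direction for traversing the path.
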(event `self.ReceiveBeginPlay`
  (bind _returnvalue (`AIBlueprintHelperLibrary.GetBlackboard` null))
  (`self.RunBehaviorTree` "/Game/AI/InfectedNPC/BT_iNPC.BT_iNPC")
  (bind _asi_npc (cast `/Game/AI/InfectedNPC/iNPC` (`self.K2_GetPawn`)))
  (bind _output_get (set `self.MyPawn` _asi_npc))
  (`BlackboardComponent.SetValueAsBool` _returnvalue "PathLooping" (`/Game/AI/PatrolPath.IsLooping` (`/Game/AI/InfectedNPC/iNPC.PatrolPath` _output_get)))
  (`BlackboardComponent.SetValueAsInt` _returnvalue "Direction" 1)
  (`BlackboardComponent.SetValueAsFloat` _returnvalue "WaitTime" (`/Game/AI/PatrolPath.WaitTime` (`/Game/AI/InfectedNPC/iNPC.PatrolPath` (`self.MyPawn`)))))

(fn `UserConstructionScript`)