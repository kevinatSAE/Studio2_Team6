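; Toilet actor that the player can interact with to take a swab.
; Overlap with the ThirdPersonCharacter enables input from player controller 0 on the actor, and leaving disables it.
; Pressing E reads IsHoldingSwab on the player pawn and prints either a swabbed message or a notice that a swab is needed, with no state change.
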(event `self.ReceiveActorBeginOverlap`
  (params (OtherActor :type "Actor Object Reference"))
  (cast `/Game/ThirdPersonBP/Blueprints/ThirdPersonCharacter` OtherActor)
  (`self.EnableInput` (`GameplayStatics.GetPlayerController` 0)))

(event `self.ReceiveActorEndOverlap`
  (params (OtherActor :type "Actor Object Reference"))
  (cast `/Game/ThirdPersonBP/Blueprints/ThirdPersonCharacter` OtherActor)
  (`self.DisableInput` (`GameplayStatics.GetPlayerController` 0)))

(event `Key|E`
  (params (Key :type "Key Structure"))
  (:`Pressed`
    (bind _asthird_person_character (cast `/Game/ThirdPersonBP/Blueprints/ThirdPersonCharacter` (`GameplayStatics.GetPlayerPawn` 0)))
    (if (`/Game/ThirdPersonBP/Blueprints/ThirdPersonCharacter.IsHoldingSwab` _asthird_person_character)
      (`KismetSystemLibrary.PrintString` "swabbed")
      (else
        (`KismetSystemLibrary.PrintString` "you need to be holding a swab")))))

(fn `UserConstructionScript`)