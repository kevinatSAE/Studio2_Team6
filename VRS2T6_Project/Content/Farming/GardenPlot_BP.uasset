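; Garden plot actor that, once composted, seeded and watered, reveals a static mesh and infects the player.
; Overlap by the ThirdPersonCharacter toggles the plot's input, though no input handlers or setters for the three state flags appear here.
; Tick polls the flags behind a Delay, then a DoOnce waits briefly, shows the mesh, calls AddInfection and swaps the player's material to polished walnut.
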(event `self.ReceiveActorBeginOverlap`
  (params (OtherActor :type "Actor Object Reference"))
  (cast `/Game/ThirdPersonBP/Blueprints/ThirdPersonCharacter` OtherActor)
  (`self.EnableInput` (`GameplayStatics.GetPlayerController` 0)))

(event `self.ReceiveActorEndOverlap`
  (params (OtherActor :type "Actor Object Reference"))
  (cast `/Game/ThirdPersonBP/Blueprints/ThirdPersonCharacter` OtherActor)
  (`self.DisableInput` (`GameplayStatics.GetPlayerController` 0)))

(event `self.ReceiveTick`
  (params (DeltaSeconds :type "Float (single-precision)"))
  (`KismetSystemLibrary.Delay` (+ (`self.Tick`) DeltaSeconds))
  (if (and (`self.IsComposted`) (`self.IsSeeded`) (`self.IsWatered`))
    (`/Engine/EditorBlueprintResources/StandardMacros.DoOnce` false
      (:`Completed`
        (`KismetSystemLibrary.Delay` 1.0)
        (`SceneComponent.SetVisibility` (`/Game/Farming/Plant_BP_2.StaticMesh` (`self.Object`)) true false)
        (bind _asthird_person_character (cast `/Game/ThirdPersonBP/Blueprints/ThirdPersonCharacter` (`GameplayStatics.GetPlayerPawn` 0)))
        (`/Game/ThirdPersonBP/Blueprints/ThirdPersonCharacter.Add Infection` _asthird_person_character)
        (`PrimitiveComponent.SetMaterial` (`Character.Mesh` _asthird_person_character) 0 "/Game/StarterContent/Materials/M_Wood_Floor_Walnut_Polished.M_Wood_Floor_Walnut_Polished")))))

(fn `UserConstructionScript`)