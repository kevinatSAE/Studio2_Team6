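; VR gym equipment actor that the player can clean and exercise on, using the MotionControllerPawn.
; Overlap enables input; holding a towel marks it cleaned and briefly shows a hygiene fun fact.
; The TeleportRight press flip-flops between locking the pawn at a fixed exercise spot with the gym widget and releasing it.
; A Lifting event grades reps by GymWidget animation timing and barbell overlap, only printing the result.
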(event `self.ReceiveActorBeginOverlap`
  (params (OtherActor :type "Actor Object Reference"))
  (bind _asmotion_controller_pawn (cast `/Game/VirtualRealityBP/Blueprints/MotionControllerPawn` OtherActor))
  (`self.EnableInput` (`GameplayStatics.GetPlayerController` 0))
  (if (`/Game/VirtualRealityBP/Blueprints/MotionControllerPawn.HoldingTowel` _asmotion_controller_pawn)
    (`KismetSystemLibrary.PrintString` "object cleaned")
    (set `self.isCleaned` true)
    (set `/Game/VirtualRealityBP/Blueprints/MotionControllerPawn.FunfactText` "Did you know: \n70 per cent of gym equipment have germs that caused skin infections and illnesses" _asmotion_controller_pawn)
    (bind _funfactwidget (`/Game/VirtualRealityBP/Blueprints/MotionControllerPawn.FunfactWidget` _asmotion_controller_pawn))
    (`SceneComponent.SetVisibility` _funfactwidget true false)
    (`KismetSystemLibrary.Delay` 5.0)
    (`SceneComponent.SetVisibility` _funfactwidget false false)))

(event `InputAction|TeleportRight`
  (params (Key :type "Key Structure"))
  (:`Pressed`
    (`/Engine/EditorBlueprintResources/StandardMacros.FlipFlop`
      (:`A`
        (bind _asmotion_controller_pawn (cast `/Game/VirtualRealityBP/Blueprints/MotionControllerPawn` (`GameplayStatics.GetPlayerPawn` 0)))
        (`SceneComponent.K2_SetWorldLocationAndRotation` (`Actor.RootComponent` _asmotion_controller_pawn) (-300.0 -311.0 251.0) (struct :`Pitch` 90.0 :`Yaw` 90.0) false false)
        (set `/Game/VirtualRealityBP/Blueprints/MotionControllerPawn.CanMove` false _asmotion_controller_pawn)
        (`SceneComponent.SetVisibility` (`/Game/VirtualRealityBP/Blueprints/MotionControllerPawn.GymingWidget` _asmotion_controller_pawn) true false))
      (:`B`
        (bind _asmotion_controller_pawn_2 (cast `/Game/VirtualRealityBP/Blueprints/MotionControllerPawn` (`GameplayStatics.GetPlayerPawn` 0)))
        (`SceneComponent.K2_SetWorldLocationAndRotation` :`self` (`Actor.RootComponent` _asmotion_controller_pawn_2) :`NewLocation` (-300.0 -311.0 251.0))
        (set `/Game/VirtualRealityBP/Blueprints/MotionControllerPawn.CanMove` true _asmotion_controller_pawn_2)
        (`SceneComponent.SetVisibility` (`/Game/VirtualRealityBP/Blueprints/MotionControllerPawn.GymingWidget` _asmotion_controller_pawn_2) false false)
        (`SceneComponent.SetVisibility` (`/Game/VirtualRealityBP/Blueprints/MotionControllerPawn.FunfactWidget` _asmotion_controller_pawn_2) false false)))))

(event `Lifting`
  (bind _gymwidget (`self.GymWidget`))
  (bind _animationtime (`/Game/Widgets/GymWidget.AnimationTime` _gymwidget))
  (`/Engine/EditorBlueprintResources/StandardMacros.IsValid` _gymwidget
    (:`Is Valid`
      (if (and (>= _animationtime 0.75) (<= _animationtime 1.3) (`self.BarbellisIn`))
        (`KismetSystemLibrary.PrintString` "good")
        (else
          (`KismetSystemLibrary.PrintString` "false"))))))

(event `self.ReceiveActorEndOverlap`
  (params (OtherActor :type "Actor Object Reference"))
  (bind _asmotion_controller_pawn (cast `/Game/VirtualRealityBP/Blueprints/MotionControllerPawn` OtherActor))
  (`SceneComponent.SetVisibility` (`/Game/VirtualRealityBP/Blueprints/MotionControllerPawn.GymingWidget` _asmotion_controller_pawn) false false)
  (`SceneComponent.SetVisibility` (`/Game/VirtualRealityBP/Blueprints/MotionControllerPawn.FunfactWidget` _asmotion_controller_pawn) false false))

(event `self.BarbellCheck.OnComponentBeginOverlap`
  (params (OverlappedComponent :type "PrimitiveComponent Object Reference") (OtherActor :type "Actor Object Reference") (OtherComp :type "PrimitiveComponent Object Reference") (OtherBodyIndex :type Integer) (bFromSweep :type Boolean) (SweepResult :type "HitResult Structure (by ref)"))
  (cast `/Game/Assets/Barbell_BP` OtherActor)
  (set `self.Barbell` null)
  (set `self.BarbellisIn` true))

(event `self.BarbellCheck.OnComponentEndOverlap`
  (params (OverlappedComponent :type "PrimitiveComponent Object Reference") (OtherActor :type "Actor Object Reference") (OtherComp :type "PrimitiveComponent Object Reference") (OtherBodyIndex :type Integer))
  (cast `/Game/Assets/Barbell_BP` OtherActor)
  (set `self.BarbellisIn` false))

(event `self.Box.OnComponentBeginOverlap`
  (params (OverlappedComponent :type "PrimitiveComponent Object Reference") (OtherActor :type "Actor Object Reference") (OtherComp :type "PrimitiveComponent Object Reference") (OtherBodyIndex :type Integer) (bFromSweep :type Boolean) (SweepResult :type "HitResult Structure (by ref)"))
  (cast `/Game/VirtualRealityBP/Blueprints/MotionControllerPawn` OtherActor))

(event `self.Box.OnComponentEndOverlap`
  (params (OverlappedComponent :type "PrimitiveComponent Object Reference") (OtherActor :type "Actor Object Reference") (OtherComp :type "PrimitiveComponent Object Reference") (OtherBodyIndex :type Integer))
  (cast `/Game/VirtualRealityBP/Blueprints/MotionControllerPawn` OtherActor))

(fn `UserConstructionScript`)