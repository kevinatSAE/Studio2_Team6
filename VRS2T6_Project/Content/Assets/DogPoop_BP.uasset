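; Dog poop actor for a motion-controller game that infects the player on contact and can be picked up.
; Overlap with MotionControllerPawn calls PlayerInfected, and end overlap calls PlayerNotInfected.
; Overlap with Shovel_BP attaches the shovel's Head component to the poop's root with relative transform rules.
; Pickup, called by BP_MotionController, attaches the root to the given component, and Drop detaches it, both keeping world transform.
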(event `self.ReceiveActorBeginOverlap`
  (params (OtherActor :type "Actor Object Reference"))
  (bind _asmotion_controller_pawn (cast `/Game/VirtualRealityBP/Blueprints/MotionControllerPawn` OtherActor)
    (:`then`
      (`KismetSystemLibrary.PrintString` "overlap gonna infect")
      (`/Game/VirtualRealityBP/Blueprints/MotionControllerPawn.PlayerInfected` _asmotion_controller_pawn))
    (:`CastFailed`
      (bind _asshovel_bp (cast `/Game/Assets/Shovel_BP` OtherActor))
      (`SceneComponent.K2_AttachToComponent` (`/Game/Assets/Shovel_BP.head` _asshovel_bp) (`self.DefaultSceneRoot`) "None" "KeepRelative" "KeepRelative" "KeepRelative" true))))

(event `self.ReceiveActorEndOverlap`
  (params (OtherActor :type "Actor Object Reference"))
  (bind _asmotion_controller_pawn (cast `/Game/VirtualRealityBP/Blueprints/MotionControllerPawn` OtherActor))
  (`/Game/VirtualRealityBP/Blueprints/MotionControllerPawn.PlayerNotInfected` _asmotion_controller_pawn))

(event `/Game/VirtualRealityBP/Blueprints/PickupActorInterface.Pickup`
  (params (AttachTo :type "SceneComponent Object Reference"))
  (`SceneComponent.K2_AttachToComponent` (`self.K2_GetRootComponent`) AttachTo "None" "KeepWorld" "KeepWorld" "KeepWorld" false))

(event `/Game/VirtualRealityBP/Blueprints/PickupActorInterface.Drop`
  (`self.K2_DetachFromActor` "KeepWorld" "KeepWorld" "KeepWorld"))

(fn `UserConstructionScript`)