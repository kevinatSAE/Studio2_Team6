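; Petri dish actor that shows its Bacteria component when the player presses E nearby after swabbing the keyboard.
; Overlap begin and end with the ThirdPersonCharacter enable and disable the dish's input.
; E checks KeyboardSwabbed on the character reference from the end-overlap cast, then reveals the bacteria after a one-second delay with a debug print.
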(event `self.ReceiveActorBeginOverlap`
  (params (OtherActor :type "Actor Object Reference"))
  (cast `/Game/ThirdPersonBP/Blueprints/ThirdPersonCharacter` OtherActor)
  (`self.EnableInput` (`GameplayStatics.GetPlayerController` 0)))

(event `self.ReceiveActorEndOverlap`
  (params (OtherActor :type "Actor Object Reference"))
  (bind _asthird_person_character (cast `/Game/ThirdPersonBP/Blueprints/ThirdPersonCharacter` OtherActor))
  (`self.DisableInput` (`GameplayStatics.GetPlayerController` 0)))

(event `Key|E`
  (params (Key :type "Key Structure"))
  (:`Pressed`
    (if (`/Game/ThirdPersonBP/Blueprints/ThirdPersonCharacter.KeyboardSwabbed` (stale `self.ReceiveActorEndOverlap` _asthird_person_character))
      (`KismetSystemLibrary.Delay` 1.0)
      (`SceneComponent.SetVisibility` (`self.Bacteria`) true false)
      (`KismetSystemLibrary.PrintString` "Bacteria spawned"))))

(fn `UserConstructionScript`)