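; Barbell actor for the gym that can be picked up by a VR motion controller and detected by gym equipment.
; Overlap events set the BarbellisIn flag on any overlapping GymObject_BP, printing it on entry and clearing it on exit.
; Pickup disables physics and attaches the root to the controller's Barbell socket, keeping world transform.
; Drop detaches it but leaves physics disabled, so it stays where released.
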(event `self.ReceiveActorBeginOverlap`
  (params (OtherActor :type "Actor Object Reference"))
  (bind _asgym_object_bp (cast `/Game/Assets/Gym/GymObject_BP` OtherActor))
  (bind _output_get (set `/Game/Assets/Gym/GymObject_BP.BarbellisIn` true _asgym_object_bp))
  (`KismetSystemLibrary.PrintString` (`KismetStringLibrary.Conv_BoolToString` _output_get)))

(event `self.ReceiveActorEndOverlap`
  (params (OtherActor :type "Actor Object Reference"))
  (bind _asgym_object_bp (cast `/Game/Assets/Gym/GymObject_BP` OtherActor))
  (set `/Game/Assets/Gym/GymObject_BP.BarbellisIn` false _asgym_object_bp))

(event `/Game/VirtualRealityBP/Blueprints/PickupActorInterface.Pickup`
  (params (AttachTo :type "SceneComponent Object Reference"))
  (`PrimitiveComponent.SetSimulatePhysics` (`self.StaticMesh`) false)
  (`SceneComponent.K2_AttachToComponent` (`self.K2_GetRootComponent`) AttachTo "Barbell" "KeepWorld" "KeepWorld" "KeepWorld" false))

(event `/Game/VirtualRealityBP/Blueprints/PickupActorInterface.Drop`
  (`PrimitiveComponent.SetSimulatePhysics` (`self.StaticMesh`) false)
  (`self.K2_DetachFromActor` "KeepWorld" "KeepWorld" "KeepWorld"))

(fn `UserConstructionScript`)