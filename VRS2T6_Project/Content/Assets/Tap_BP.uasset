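; VR hand-washing tap that reacts when a motion controller overlaps it and lowers the player's infection.
; On begin overlap it plays a faucet sound, flashes a P_Sparks splash emitter, briefly spawns a scaled-down Soap_BP at the drop point, then calls MinusInfection on the MotionControllerPawn.
; On end overlap it shows a hand-washing fun fact on the pawn's widget for a few seconds.
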(event `self.ReceiveActorBeginOverlap`
  (params (OtherActor :type "Actor Object Reference"))
  (cast `/Game/VirtualRealityBP/Blueprints/BP_MotionController` OtherActor)
  (bind _asmotion_controller_pawn (cast `/Game/VirtualRealityBP/Blueprints/MotionControllerPawn` (`GameplayStatics.GetPlayerPawn` 0)))
  (`GameplayStatics.PlaySoundAtLocation` "/Game/Sounds/zapsplat_household_tap_faucet_basin_bathroom_turn_on_run_short_drain_no_plug_43445.zapsplat_household_tap_faucet_basin_bathroom_turn_on_run_short_drain_no_plug_43445" (`self.K2_GetActorLocation`) (struct) 1.0 1.0 0.0 null null null)
  (bind _returnvalue (`GameplayStatics.SpawnEmitterAttached` "/Game/StarterContent/Particles/P_Sparks.P_Sparks" (`self.Splash`) "None" (0.0 0.0 -10.0)))
  (`KismetSystemLibrary.Delay` 0.2)
  (`ActorComponent.K2_DestroyComponent` _returnvalue)
  (bind _returnvalue_2 (`|SpawnActorFromClass` "/Game/Assets/Soap_BP.Soap_BP_C" (`KismetMathLibrary.MakeTransform` (+ (`SceneComponent.K2_GetComponentLocation` (`self.Drop`)) (0.0 0.0 -10.0)) (struct) (0.125 0.083333 0.0625)) "Undefined" "OverrideRootScale" (`ActorComponent.GetOwner` (`self.Box`)) null))
  (`KismetSystemLibrary.Delay` 0.5)
  (`self.K2_DestroyActor` _returnvalue_2)
  (`/Game/VirtualRealityBP/Blueprints/MotionControllerPawn.Minus Infection` _asmotion_controller_pawn))

(event `self.ReceiveActorEndOverlap`
  (params (OtherActor :type "Actor Object Reference"))
  (cast `/Game/VirtualRealityBP/Blueprints/BP_MotionController` OtherActor)
  (`KismetSystemLibrary.PrintString` "end overlap")
  (bind _asmotion_controller_pawn (cast `/Game/VirtualRealityBP/Blueprints/MotionControllerPawn` (`GameplayStatics.GetPlayerPawn` 0)))
  (set `/Game/VirtualRealityBP/Blueprints/MotionControllerPawn.FunfactText` "Did you know: \n1 in 5 people don't wash their hands!" _asmotion_controller_pawn)
  (bind _funfactwidget (`/Game/VirtualRealityBP/Blueprints/MotionControllerPawn.FunfactWidget` _asmotion_controller_pawn))
  (`SceneComponent.SetVisibility` _funfactwidget true false)
  (`KismetSystemLibrary.Delay` 5.0)
  (`SceneComponent.SetVisibility` _funfactwidget false false))

(fn `UserConstructionScript`)