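; Toilet actor for a swabbing task, which records on the player pawn that the toilet has been swabbed if a swab is held.
; Overlap by a MotionControllerPawn enables input and immediately sets ToiletSwabbed when that pawn holds a swab.
; A separate E key path does the same for a ThirdPersonCharacter, printing success or a need-a-swab message.
; End overlap does nothing, and the DisableInput call is never executed.
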(event `self.ReceiveActorBeginOverlap`
  (params (OtherActor :type "Actor Object Reference"))
  (bind _asmotion_controller_pawn (cast `/Game/VirtualRealityBP/Blueprints/MotionControllerPawn` OtherActor))
  (`self.EnableInput` null)
  (if (`/Game/VirtualRealityBP/Blueprints/MotionControllerPawn.isHoldingSwab` _asmotion_controller_pawn)
    (set `/Game/VirtualRealityBP/Blueprints/MotionControllerPawn.ToiletSwabbed` true _asmotion_controller_pawn)))

(event `self.ReceiveActorEndOverlap`
  (params (OtherActor :type "Actor Object Reference")))

(event `Key|E`
  (params (Key :type "Key Structure"))
  (:`Pressed`
    (bind _asthird_person_character (cast `/Game/ThirdPersonBP/Blueprints/ThirdPersonCharacter` (`GameplayStatics.GetPlayerPawn` 0)))
    (if (`/Game/ThirdPersonBP/Blueprints/ThirdPersonCharacter.IsHoldingSwab` _asthird_person_character)
      (`KismetSystemLibrary.PrintString` "swabbed")
      (set `/Game/ThirdPersonBP/Blueprints/ThirdPersonCharacter.ToiletSwabbed` true _asthird_person_character)
      (else
        (`KismetSystemLibrary.PrintString` "you need to be holding a swab")))))

(fn `UserConstructionScript`)