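; Swab Blueprint: a VR swab prop that the motion controllers pick up and drop.
; Pickup disables physics, snaps it to the hand_rSocket of the given component and sets IsHoldingSwab on the MotionControllerPawn.
; Drop detaches it at its world position and rotation and clears the flag through the pawn reference cast in Pickup.
; Drop also leaves physics disabled, so the released swab does not fall under simulation.
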(event `/Game/VirtualRealityBP/Blueprints/PickupActorInterface.Pickup`
  (params (AttachTo :type "SceneComponent Object Reference"))
  (`PrimitiveComponent.SetSimulatePhysics` (`self.r`) false)
  (`SceneComponent.K2_AttachToComponent` (`self.K2_GetRootComponent`) AttachTo "hand_rSocket" "SnapToTarget" "SnapToTarget" "KeepWorld" false)
  (bind _asmotion_controller_pawn (cast `/Game/VirtualRealityBP/Blueprints/MotionControllerPawn` (`GameplayStatics.GetPlayerPawn` 0)))
  (set `/Game/VirtualRealityBP/Blueprints/MotionControllerPawn.isHoldingSwab` true _asmotion_controller_pawn))

(event `/Game/VirtualRealityBP/Blueprints/PickupActorInterface.Drop`
  (`PrimitiveComponent.SetSimulatePhysics` (`self.r`) false)
  (`self.K2_DetachFromActor` "KeepWorld" "KeepWorld" "KeepWorld")
  (set `/Game/VirtualRealityBP/Blueprints/MotionControllerPawn.isHoldingSwab` false (stale `/Game/VirtualRealityBP/Blueprints/PickupActorInterface.Pickup` _asmotion_controller_pawn)))

(fn `UserConstructionScript`)