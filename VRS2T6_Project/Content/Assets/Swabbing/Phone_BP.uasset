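; Phone actor for a swabbing task that registers when the motion controller pawn swabs it.
; On overlap with the pawn it enables player input and sets the pawn's PhoneSwabbed flag if a swab is held.
; The E key only prints whether a swab is held, without setting the flag.
; End overlap does nothing after its cast, and the DisableInput node is unconnected, so input stays enabled.
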(event `self.ReceiveActorBeginOverlap`
  (params (OtherActor :type "Actor Object Reference"))
  (bind _asmotion_controller_pawn (cast `/Game/VirtualRealityBP/Blueprints/MotionControllerPawn` OtherActor))
  (`self.EnableInput` (`GameplayStatics.GetPlayerController` 0))
  (if (`/Game/VirtualRealityBP/Blueprints/MotionControllerPawn.isHoldingSwab` _asmotion_controller_pawn)
    (set `/Game/VirtualRealityBP/Blueprints/MotionControllerPawn.PhoneSwabbed` true _asmotion_controller_pawn)))

(event `self.ReceiveActorEndOverlap`
  (params (OtherActor :type "Actor Object Reference"))
  (cast `/Game/VirtualRealityBP/Blueprints/MotionControllerPawn` OtherActor))

(event `Key|E`
  (params (Key :type "Key Structure"))
  (:`Pressed`
    (bind _asmotion_controller_pawn (cast `/Game/VirtualRealityBP/Blueprints/MotionControllerPawn` (`GameplayStatics.GetPlayerPawn` 0)))
    (if (`/Game/VirtualRealityBP/Blueprints/MotionControllerPawn.isHoldingSwab` _asmotion_controller_pawn)
      (`KismetSystemLibrary.PrintString` "swabbed")
      (else
        (`KismetSystemLibrary.PrintString` "you need to be holding a swab")))))

(fn `UserConstructionScript`)